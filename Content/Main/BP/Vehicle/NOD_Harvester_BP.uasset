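; NOD Harvester vehicle Blueprint that runs a Tiberium harvest-and-unload loop between a harvest point and a refinery.
; RenegadeHarvesterCombat events start timed harvesting and unloading, each with a spawned particle effect, then send the vehicle to the other destination.
; Undocking also clears the unload effect and restarts the cycle.
; Tick uses paired DoOnce gates to swap static and moving track materials when speed crosses a threshold.
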(event OnHarvestPointArrived(RenegadeHarvesterCombat)
  (params (HarvestPoint :type Renegade%20Harvest%20Point%20Object%20Reference))
  (bind _renegadeharvestercombat (Variables|Default|GetRenegadeHarvesterCombat))
  (bind _renegadeharvestercombat_2 (Variables|Default|GetRenegadeHarvesterCombat))
  (Class|RenegadeHarvesterCombatComponent|StartHarvesting _renegadeharvestercombat)
  (Variables|Default|SetIsHarvesting true)
  (bind _returnvalue (Effects|SpawnEmitteratLocation "/Game/Utilities/VectorParticles/Particles/P_VectorField15.P_VectorField15" (Transformation|GetWorldLocation (Variables|Default|GetScene)) "0.000000,0.000000,-88.716525" "0.469677,0.469677,0.469677"))
  (Variables|Default|SetTiberiumHarvetParticle _returnvalue)
  (Development|PrintString "NOD Harvester Is Now Harvesting")
  (Utilities|FlowControl|Delay 8.0)
  (Class|RenegadeHarvesterCombatComponent|EndHarvesting _renegadeharvestercombat)
  (Variables|Default|SetIsHarvesting false)
  (bind _tiberiumharvetparticle (Variables|Default|GetTiberiumHarvetParticle)
    (:then
      (Components|DestroyComponent _tiberiumharvetparticle))
    (:else
      _))
  (Variables|Default|SetTiberiumHarvetParticle 0)
  (Class|RenegadeHarvesterCombatComponent|GotoRefineryDockPoint _renegadeharvestercombat_2)
  (Development|PrintString "NOD Harvester has stoped Harvesting and returning to dock station")
  (Class|RenegadeHarvesterCombatComponent|MarkReturningtoRefinery _renegadeharvestercombat_2))

(event OnRefineryDocked(RenegadeHarvesterCombat)
  (bind _renegadeharvestercombat (Variables|Default|GetRenegadeHarvesterCombat))
  (Class|RenegadeHarvesterCombatComponent|StartRefineryUnloading _renegadeharvestercombat)
  (Development|PrintString "NOD Harvester is unloading cargo at dock station")
  (bind _returnvalue (Effects|SpawnEmitteratLocation "/Game/Utilities/VectorParticles/Particles/P_VectorField14.P_VectorField14" (Transformation|GetWorldLocation (Variables|Default|GetScene1)) "0.000000,0.000000,-88.716525" "0.318736,0.318736,0.318736"))
  (Variables|Default|SetUnloadTiberiumParticle _returnvalue)
  (Utilities|FlowControl|Delay 1e+01)
  (Class|RenegadeHarvesterCombatComponent|EndRefineryUnloading _renegadeharvestercombat)
  (bind _unloadtiberiumparticle (Variables|Default|GetUnloadTiberiumParticle)
    (:then
      (Components|DestroyComponent _unloadtiberiumparticle))
    (:else
      _))
  (Variables|Default|SetUnloadTiberiumParticle 0)
  (Development|PrintString "NOD Harvester is restarting its harvest cycle.")
  (CallFunction|RestartHarvesterCycle))

(event OnRefineryUndocked(RenegadeHarvesterCombat)
  (bind _unloadtiberiumparticle (Variables|Default|GetUnloadTiberiumParticle)
    (:then
      (Components|DestroyComponent _unloadtiberiumparticle))
    (:else
      _))
  (Variables|Default|SetUnloadTiberiumParticle 0)
  (Development|PrintString "NOD Harvester is restarting its harvest cycle.")
  (CallFunction|RestartHarvesterCycle))

(event Custom|RestartHarvesterCycle
  (Class|RenegadeHarvesterCombatComponent|GotoHarvestPoint (Variables|Default|GetRenegadeHarvesterCombat)))

(event Collision|EventActorBeginOverlap
  (params (OtherActor :type Actor%20Object%20Reference)))

(event EventTick
  (params (DeltaSeconds :type Float%20%28single-precision%29))
  (bind _mesh (Variables|Character|GetMesh))
  (if (< (Math|Vector|VectorLength (Variables|/Script/Engine.MovementComponent|GetVelocity (Variables|Character|GetCharacterMovement))) 5e+01)
    (Utilities|FlowControl|DoOnce false :!label _label
      (:Completed
        (Rendering|Material|SetMaterial _mesh 1 "/Game/Main/SK/Vehicle/Harvester/LightTank_Tracks_D_Mat.LightTank_Tracks_D_Mat")
        (goto _label_2 Reset)))
    (else
      (Utilities|FlowControl|DoOnce false :!label _label_2
        (:Completed
          (Rendering|Material|SetMaterial _mesh 1 "/Game/Main/SK/Vehicle/Harvester/LightTank_TracksMoving_D_Mat.LightTank_TracksMoving_D_Mat")
          (goto _label Reset))))))

(event EventBeginPlay)

(fn ConstructionScript)