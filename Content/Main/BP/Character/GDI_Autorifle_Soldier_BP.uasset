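; GDI autorifle soldier character that fights as either an AI path follower or a player-controlled combatant.
; RenegadeSoldierCombat events drive muzzle flash, rifle sound, blood on Nod autorifle soldier hits, and spline path resumption after combat or respawn.
; Player input handles firing and aiming, which cancels sprint.
; Weapon changes swap mesh, materials, scale and anim class between rifle and pistol, nudging the muzzle by world-space offsets.
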(event OnShotFired(RenegadeSoldierCombat)
  (params (TraceStart :type Vector :default "0, 0, 0") (TraceEnd :type Vector :default "0, 0, 0") (bBlockingHit :type Boolean) (HitResult :type Hit%20Result%20Structure%20%28by%20ref%29))
  (bind _muzzle (Variables|Default|GetMuzzle))
  (bind _muzzle_2 (Variables|Default|GetMuzzle)
    (:then
      (if (Variables|/Script/RenegadeSoldierCombat.RenegadeSoldierCombatComponent|GetbPlayerControlledCombat (Variables|Default|GetRenegadeSoldierCombat))
        (Effects|SpawnEmitterAttached "/Game/Utilities/ShooterVFXVariety/Particles/P_Shotgun_MuzzleFlash1.P_Shotgun_MuzzleFlash1" _muzzle "" (Transformation|GetWorldLocation _muzzle_2) (Math|Rotator|FindLookatRotation (Transformation|GetWorldLocation _muzzle_2) TraceEnd) "0.500000,0.500000,0.500000" "KeepWorldPosition")
        (else
          (Effects|SpawnEmitterAttached "/Game/Utilities/ShooterVFXVariety/Particles/P_Shotgun_MuzzleFlash.P_Shotgun_MuzzleFlash" _muzzle "" (Transformation|GetWorldLocation _muzzle_2) (Math|Rotator|FindLookatRotation (Transformation|GetWorldLocation _muzzle_2) TraceEnd) "1.000000,1.000000,1.000000" "KeepWorldPosition")))
      (Audio|PlaySoundatLocation "/Game/Main/Sound/Weapon/Autorifle/RifleFire_Cue.RifleFire_Cue" (Transformation|GetActorLocation) (Math|Rotator|FindLookatRotation (Transformation|GetWorldLocation _muzzle_2) TraceEnd) 1.0 1.0 0.0 0 0 0 0)
      (Utilities|Casting|CastToNOD_Autorifle_Soldier_BP (.HitActor (Collision|BreakHitResult HitResult)))
      (Effects|SpawnEmitteratLocation "/Game/Utilities/ShooterVFXVariety/BloodVFX/Particles/Cascade/Real/P_Blood_BulletHit.P_Blood_BulletHit" TraceEnd (Math|Rotator|FindLookatRotation (Transformation|GetWorldLocation _muzzle_2) TraceEnd) "2.000000,2.000000,2.000000"))
    (:else)))

(event OnCombatEnded(RenegadeSoldierCombat)
  (params (PreviousTarget :type Actor%20Object%20Reference) (ResumeFromLocation :type Vector :default "0, 0, 0"))
  (Class|RenegadeSplineFollowerComponent|ResumeFollowing (Variables|Default|GetRenegadeSplineFollower) true))

(event OnPlayerWeaponChanged(RenegadeSoldierCombat)
  (params (PreviousWeapon :type ERenegadePlayerWeaponSlot%20Enum :default "AutomaticRifle") (NewWeapon :type ERenegadePlayerWeaponSlot%20Enum :default "AutomaticRifle"))
  (bind _sk_autorifle_1p_newrig (Variables|Default|GetSK_AutoRifle_1P_NewRig))
  (bind _muzzle (Variables|Default|GetMuzzle))
  (bind _muzzle_2 (Variables|Default|GetMuzzle))
  (if (Utilities|Enum|Equal(Enum) NewWeapon "AutomaticRifle")
    (Components|SkeletalMesh|SetSkeletalMeshAsset _sk_autorifle_1p_newrig "/Game/Main/SK/Weapons/AutoRifle/SK_AutoRifle_1P_NewRig.SK_AutoRifle_1P_NewRig")
    (Rendering|Material|SetMaterial _sk_autorifle_1p_newrig 0 "/Game/Main/SK/Weapons/AutoRifle/TexMat/T_AutoRifle_Nod_D_Mat.T_AutoRifle_Nod_D_Mat")
    (Rendering|Material|SetMaterial _sk_autorifle_1p_newrig 1 "/Game/Main/Mesh/Buildings/NOD/Airstrip/FlashingLight_T_Mat.FlashingLight_T_Mat")
    (Rendering|Material|SetMaterial _sk_autorifle_1p_newrig 2 "/Game/Main/Mesh/Buildings/NOD/PowerPlant/BlinkingGreenLights_M.BlinkingGreenLights_M")
    (Rendering|Material|SetMaterial _sk_autorifle_1p_newrig 3 "/Game/Main/Mesh/Buildings/NOD/Airstrip/FlashingLight_T_Mat.FlashingLight_T_Mat")
    (Rendering|Material|SetMaterial _sk_autorifle_1p_newrig 4 "/Game/Main/Texture/Misc/SightScanline_Mat.SightScanline_Mat")
    (Components|SkeletalMesh|SetAnimInstanceClass (Variables|Character|GetMesh) "/Game/Main/SK/GDI/Havoc/SK_Havoc_AnimBP.SK_Havoc_AnimBP_C")
    (Transformation|SetWorldScale3D (Variables|Default|GetSK_AutoRifle_1P_NewRig) "4.000000,4.000000,4.000000")
    (Transformation|SetWorldLocation _muzzle (- (Transformation|GetWorldLocation _muzzle) "40.000000,0.000000,10.000000") false false)
    (elif (Utilities|Enum|Equal(Enum) NewWeapon "Pistol")
      (Components|SkeletalMesh|SetSkeletalMeshAsset _sk_autorifle_1p_newrig "/Game/Main/SK/Weapons/Pistol/SK_WP_Pistol_3P.SK_WP_Pistol_3P")
      (Rendering|Material|SetMaterial _sk_autorifle_1p_newrig 0 "/Game/Main/SK/Weapons/Pistol/Pistol_D_Mat.Pistol_D_Mat")
      (Components|SkeletalMesh|SetAnimInstanceClass (Variables|Character|GetMesh) "/Game/Main/SK/GDI/Havoc/SK_Havoc_AnimBP2.SK_Havoc_AnimBP2_C")
      (Transformation|SetWorldScale3D (Variables|Default|GetSK_AutoRifle_1P_NewRig) "2.000000,2.000000,2.000000")
      (Transformation|SetWorldLocation _muzzle_2 (+ (Transformation|GetWorldLocation _muzzle_2) "20.000000,0.000000,5.000000") false false))))

(event OnRespawned(RenegadeSoldierCombat)
  (bind _returnvalue (Class|RenegadeSplineAIBlueprintLibrary|FindNearestCompatiblePath (Transformation|GetActorLocation self) 1 "None" 0.0))
  (Class|RenegadeSplineFollowerComponent|StartFollowing (Variables|Default|GetRenegadeSplineFollower) _returnvalue true))

(event EventBeginPlay
  (bind _mesh (Variables|Character|GetMesh))
  (|CallParentFunction)
  (Utilities|FlowControl|Delay 0.2)
  (if (Class|RenegadeSoldierCombatComponent|IsPlayerControlledCombatant (Variables|Default|GetRenegadeSoldierCombat))
    (Components|SkeletalMesh|SetAnimInstanceClass _mesh "/Game/Main/SK/GDI/Havoc/SK_Havoc_AnimBP1.SK_Havoc_AnimBP1_C")
    (else
      (Components|SkeletalMesh|SetAnimInstanceClass _mesh "/Game/Main/SK/GDI/Havoc/SK_Havoc_AnimBP.SK_Havoc_AnimBP_C"))))

(event Collision|EventActorBeginOverlap
  (params (OtherActor :type Actor%20Object%20Reference))
  (|CallParentFunction OtherActor) ; This node is disabled and will not be called.\nDrag off pins to build functionality.
)

(event EventTick
  (params (DeltaSeconds :type Float%20%28single-precision%29))
  (|CallParentFunction DeltaSeconds))

(event Input|ActionEvents|InputActionFireWeapon
  (params (Key :type Key%20Structure :default "None"))
  (bind _renegadesoldiercombat (Variables|Default|GetRenegadeSoldierCombat))
  (:Pressed
    (if (Utilities|Enum|Equal(Enum) (Variables|/Script/RenegadeSoldierCombat.RenegadeSoldierCombatComponent|GetActivePlayerWeapon (Variables|Default|GetRenegadeSoldierCombat)) "AutomaticRifle")
      (if (Class|RenegadeSoldierCombatComponent|IsPlayerControlledCombatant _renegadesoldiercombat)
        (Class|RenegadeSoldierCombatComponent|PlayerStartAutomaticRifleFire _renegadesoldiercombat))
      (elif (Utilities|Enum|Equal(Enum) (Variables|/Script/RenegadeSoldierCombat.RenegadeSoldierCombatComponent|GetActivePlayerWeapon (Variables|Default|GetRenegadeSoldierCombat)) "Pistol")
        (if (Class|RenegadeSoldierCombatComponent|IsPlayerControlledCombatant _renegadesoldiercombat)
          (Class|RenegadeSoldierCombatComponent|PlayerFirePistol (Variables|Default|GetRenegadeSoldierCombat))))))
  (:Released
    (Class|RenegadeSoldierCombatComponent|PlayerStopAutomaticRifleFire _renegadesoldiercombat)))

(event Input|MouseEvents|RightMouseButton
  (params (Key :type Key%20Structure :default "None"))
  (bind _renegadesoldiercombat (Variables|Default|GetRenegadeSoldierCombat))
  (:Pressed
    (if (Variables|Default|GetIsSprinting)
      (CallFunction|StopSprinting))
    (Class|RenegadeSoldierCombatComponent|PlayerStartAiming _renegadesoldiercombat))
  (:Released
    (Class|RenegadeSoldierCombatComponent|PlayerStopAiming _renegadesoldiercombat)))

(event Input|GamepadEvents|GamepadLeftTrigger
  (params (Key :type Key%20Structure :default "None"))
  (bind _renegadesoldiercombat (Variables|Default|GetRenegadeSoldierCombat))
  (:Pressed
    (if (Variables|Default|GetIsSprinting)
      (CallFunction|StopSprinting))
    (Class|RenegadeSoldierCombatComponent|PlayerStartAiming _renegadesoldiercombat))
  (:Released
    (Class|RenegadeSoldierCombatComponent|PlayerStopAiming _renegadesoldiercombat)))

(fn ConstructionScript
  (|CallParentFunction))

(fn RotateFacingCameraView)