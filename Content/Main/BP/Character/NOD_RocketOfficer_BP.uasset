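; Nod rocket officer character Blueprint that works as a spline-following combatant and also handles player input for aiming and firing a rocket launcher.
; RenegadeSoldierCombat does the combat work, taking fire input only when player-controlled and aim input from right mouse or left trigger, which first stops sprinting.
; Its combat-ended and respawn events drive RenegadeSplineFollower to resume following or reacquire the nearest compatible path from the current location.
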(event OnCombatEnded(RenegadeSoldierCombat)
  (params (PreviousTarget :type Actor%20Object%20Reference) (ResumeFromLocation :type Vector :default "0, 0, 0"))
  (Class|RenegadeSplineFollowerComponent|ResumeFollowing (Variables|Default|GetRenegadeSplineFollower) true))

(event OnRespawned(RenegadeSoldierCombat)
  (bind _returnvalue (Class|RenegadeSplineAIBlueprintLibrary|FindNearestCompatiblePath (Transformation|GetActorLocation self) 0 "None" 0.0))
  (Class|RenegadeSplineFollowerComponent|StartFollowing (Variables|Default|GetRenegadeSplineFollower) _returnvalue true))

(event EventBeginPlay
  (|CallParentFunction) ; This node is disabled and will not be called.\nDrag off pins to build functionality.
)

(event Collision|EventActorBeginOverlap
  (params (OtherActor :type Actor%20Object%20Reference))
  (|CallParentFunction OtherActor) ; This node is disabled and will not be called.\nDrag off pins to build functionality.
)

(event EventTick
  (params (DeltaSeconds :type Float%20%28single-precision%29))
  (|CallParentFunction DeltaSeconds) ; This node is disabled and will not be called.\nDrag off pins to build functionality.
)

(event Input|ActionEvents|InputActionFireWeapon
  (params (Key :type Key%20Structure :default "None"))
  (:Pressed
    (if (Class|RenegadeSoldierCombatComponent|IsPlayerControlledCombatant (Variables|Default|GetRenegadeSoldierCombat))
      (Class|RenegadeSoldierCombatComponent|PlayerFireRocketLauncher (Variables|Default|GetRenegadeSoldierCombat)))))

(event Input|MouseEvents|RightMouseButton
  (params (Key :type Key%20Structure :default "None"))
  (bind _renegadesoldiercombat (Variables|Default|GetRenegadeSoldierCombat))
  (:Pressed
    (if (Variables|Default|GetIsSprinting)
      (CallFunction|StopSprinting))
    (Class|RenegadeSoldierCombatComponent|PlayerStartAiming _renegadesoldiercombat))
  (:Released
    (Class|RenegadeSoldierCombatComponent|PlayerStopAiming _renegadesoldiercombat)))

(event Input|GamepadEvents|GamepadLeftTrigger
  (params (Key :type Key%20Structure :default "None"))
  (bind _renegadesoldiercombat (Variables|Default|GetRenegadeSoldierCombat))
  (:Pressed
    (if (Variables|Default|GetIsSprinting)
      (CallFunction|StopSprinting))
    (Class|RenegadeSoldierCombatComponent|PlayerStartAiming _renegadesoldiercombat))
  (:Released
    (Class|RenegadeSoldierCombatComponent|PlayerStopAiming _renegadesoldiercombat)))

(fn ConstructionScript
  (|CallParentFunction))