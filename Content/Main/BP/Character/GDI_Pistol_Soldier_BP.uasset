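; GDI pistol soldier character that fights as an AI on team 1 lane paths or under player control, built on RenegadeSoldierCombat and RenegadeSplineFollower components.
; Shot events spawn a muzzle flash, scaled down for the player, plus pistol sound, and blood when hitting a NOD autorifle soldier.
; Combat end resumes path following, and respawn joins the nearest compatible path.
; Player input drives firing via the automatic-rifle functions and aiming, which cancels sprinting.
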(event OnShotFired(RenegadeSoldierCombat)
  (params (TraceStart :type Vector :default "0, 0, 0") (TraceEnd :type Vector :default "0, 0, 0") (bBlockingHit :type Boolean) (HitResult :type Hit%20Result%20Structure%20%28by%20ref%29))
  (bind _muzzle (Variables|Default|GetMuzzle))
  (bind _muzzle_2 (Variables|Default|GetMuzzle)
    (:then
      (if (Variables|/Script/RenegadeSoldierCombat.RenegadeSoldierCombatComponent|GetbPlayerControlledCombat (Variables|Default|GetRenegadeSoldierCombat))
        (Effects|SpawnEmitterAttached "/Game/Utilities/ShooterVFXVariety/Particles/P_Shotgun_MuzzleFlash1.P_Shotgun_MuzzleFlash1" _muzzle "" (Transformation|GetWorldLocation _muzzle_2) (Math|Rotator|FindLookatRotation (Transformation|GetWorldLocation _muzzle_2) TraceEnd) "0.500000,0.500000,0.500000" "KeepWorldPosition")
        (else
          (Effects|SpawnEmitterAttached "/Game/Utilities/ShooterVFXVariety/Particles/P_Shotgun_MuzzleFlash.P_Shotgun_MuzzleFlash" _muzzle "" (Transformation|GetWorldLocation _muzzle_2) (Math|Rotator|FindLookatRotation (Transformation|GetWorldLocation _muzzle_2) TraceEnd) "1.000000,1.000000,1.000000" "KeepWorldPosition")))
      (Audio|PlaySoundatLocation "/Game/Main/Sound/Weapon/Pistol/PistolFire_Cue.PistolFire_Cue" (Transformation|GetActorLocation) (Math|Rotator|FindLookatRotation (Transformation|GetWorldLocation _muzzle_2) TraceEnd) 1.0 1.0 0.0 0 0 0 0)
      (Utilities|Casting|CastToNOD_Autorifle_Soldier_BP (.HitActor (Collision|BreakHitResult HitResult)))
      (Effects|SpawnEmitteratLocation "/Game/Utilities/ShooterVFXVariety/BloodVFX/Particles/Cascade/Real/P_Blood_BulletHit.P_Blood_BulletHit" TraceEnd (Math|Rotator|FindLookatRotation (Transformation|GetWorldLocation _muzzle_2) TraceEnd) "2.000000,2.000000,2.000000"))
    (:else)))

(event OnCombatEnded(RenegadeSoldierCombat)
  (params (PreviousTarget :type Actor%20Object%20Reference) (ResumeFromLocation :type Vector :default "0, 0, 0"))
  (Class|RenegadeSplineFollowerComponent|ResumeFollowing (Variables|Default|GetRenegadeSplineFollower) true))

(event OnRespawned(RenegadeSoldierCombat)
  (bind _returnvalue (Class|RenegadeSplineAIBlueprintLibrary|FindNearestCompatiblePath (Transformation|GetActorLocation self) 1 "None" 0.0))
  (Class|RenegadeSplineFollowerComponent|StartFollowing (Variables|Default|GetRenegadeSplineFollower) _returnvalue true))

(event EventBeginPlay
  (|CallParentFunction) ; This node is disabled and will not be called.\nDrag off pins to build functionality.
)

(event Collision|EventActorBeginOverlap
  (params (OtherActor :type Actor%20Object%20Reference))
  (|CallParentFunction OtherActor) ; This node is disabled and will not be called.\nDrag off pins to build functionality.
)

(event EventTick
  (params (DeltaSeconds :type Float%20%28single-precision%29))
  (|CallParentFunction DeltaSeconds))

(event Input|ActionEvents|InputActionFireWeapon
  (params (Key :type Key%20Structure :default "None"))
  (bind _renegadesoldiercombat (Variables|Default|GetRenegadeSoldierCombat))
  (:Pressed
    (if (Class|RenegadeSoldierCombatComponent|IsPlayerControlledCombatant _renegadesoldiercombat)
      (Class|RenegadeSoldierCombatComponent|PlayerStartAutomaticRifleFire _renegadesoldiercombat)))
  (:Released
    (Class|RenegadeSoldierCombatComponent|PlayerStopAutomaticRifleFire _renegadesoldiercombat)))

(event Input|MouseEvents|RightMouseButton
  (params (Key :type Key%20Structure :default "None"))
  (bind _renegadesoldiercombat (Variables|Default|GetRenegadeSoldierCombat))
  (:Pressed
    (if (Variables|Default|GetIsSprinting)
      (CallFunction|StopSprinting))
    (Class|RenegadeSoldierCombatComponent|PlayerStartAiming _renegadesoldiercombat))
  (:Released
    (Class|RenegadeSoldierCombatComponent|PlayerStopAiming _renegadesoldiercombat)))

(event Input|GamepadEvents|GamepadLeftTrigger
  (params (Key :type Key%20Structure :default "None"))
  (bind _renegadesoldiercombat (Variables|Default|GetRenegadeSoldierCombat))
  (:Pressed
    (if (Variables|Default|GetIsSprinting)
      (CallFunction|StopSprinting))
    (Class|RenegadeSoldierCombatComponent|PlayerStartAiming _renegadesoldiercombat))
  (:Released
    (Class|RenegadeSoldierCombatComponent|PlayerStopAiming _renegadesoldiercombat)))

(fn ConstructionScript
  (|CallParentFunction))

(fn RotateFacingCameraView)